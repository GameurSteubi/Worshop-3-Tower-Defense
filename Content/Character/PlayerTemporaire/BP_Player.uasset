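; Player pawn for a tile-based building game with towers, sawmills and mines, handling movement, mouse look and toggles for the shop, pause and tower upgrade menus.
; Shop selection functions fill one inventory array, and clicking places that building.
; Placement traces from the cursor to a tagged tile, checks and updates its OCCUPY state, spawns the building and registers it in LevelInformation.
; The pause menu only changes input mode, as the SetGamePaused calls are unconnected.
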(event `self.ReceiveBeginPlay`
  (set `PlayerController.bShowMouseCursor` true (`GameplayStatics.GetPlayerController` 0)))

(event `EnhancedInput|/Game/ControlTemporaire/Input/IA_Shop`
  (params (ActionValue :type Boolean) (ElapsedSeconds :type "Float (double-precision)") (TriggeredSeconds :type "Float (double-precision)") (InputAction :type "InputAction Object Reference" :default "/Game/ControlTemporaire/Input/IA_Shop.IA_Shop"))
  (:`Started`
    (`self.Toggle Shop`)))

(event `EnhancedInput|/Game/ControlTemporaire/Input/IA_SecondaryAction`
  (params (ActionValue :type Boolean) (ElapsedSeconds :type "Float (double-precision)") (TriggeredSeconds :type "Float (double-precision)") (InputAction :type "InputAction Object Reference" :default "/Game/ControlTemporaire/Input/IA_SecondaryAction.IA_SecondaryAction"))
  (:`Started`
    (`self.Toggle Upgrade UI`)))

(event `EnhancedInput|/Game/ControlTemporaire/Input/IA_Look`
  (params (ActionValue :type "Vector2D Structure") (ElapsedSeconds :type "Float (double-precision)") (TriggeredSeconds :type "Float (double-precision)") (InputAction :type "InputAction Object Reference" :default "/Game/ControlTemporaire/Input/IA_Look.IA_Look"))
  (:`Triggered`
    (`self.Look` ActionValue)))

(event `EnhancedInput|/Game/ControlTemporaire/Input/IA_Pause`
  (params (ActionValue :type Boolean) (ElapsedSeconds :type "Float (double-precision)") (TriggeredSeconds :type "Float (double-precision)") (InputAction :type "InputAction Object Reference" :default "/Game/ControlTemporaire/Input/IA_Pause.IA_Pause"))
  (:`Started`
    (`self.Toggle Pause`)))

(event `EnhancedInput|/Game/ControlTemporaire/Input/IA_Move`
  (params (ActionValue :type "Vector2D Structure") (ElapsedSeconds :type "Float (double-precision)") (TriggeredSeconds :type "Float (double-precision)") (InputAction :type "InputAction Object Reference" :default "/Game/ControlTemporaire/Input/IA_Move.IA_Move"))
  (:`Triggered`
    (`self.Move` ActionValue)))

(event `Move`
  (params (Value :type "Vector2D Structure"))
  (bind (_returnvalue_roll _returnvalue_pitch _returnvalue_yaw) (`KismetMathLibrary.BreakRotator` (`self.GetControlRotation`)))
  (`self.AddMovementInput` (`KismetMathLibrary.GetRightVector` (`KismetMathLibrary.MakeRotator` 0.0 0.0 _returnvalue_yaw)) Value_X)
  (`self.AddMovementInput` (`KismetMathLibrary.GetForwardVector` (`KismetMathLibrary.MakeRotator` 0.0 0.0 _returnvalue_yaw)) Value_Y))

(event `Look`
  (params (Value :type "Vector2D Structure"))
  (`self.AddControllerYawInput` Value_X)
  (`self.AddControllerPitchInput` Value_Y))

(event `EnhancedInput|/Game/ControlTemporaire/Input/IA_Click`
  (params (ActionValue :type Boolean) (ElapsedSeconds :type "Float (double-precision)") (TriggeredSeconds :type "Float (double-precision)") (InputAction :type "InputAction Object Reference" :default "/Game/ControlTemporaire/Input/IA_Click.IA_Click"))
  (:`Started`
    (`self.Select Or Place Building`)))

(event `Toggle Pause`
  (bind _returnvalue (`GameplayStatics.GetPlayerController` 0))
  (bind _pause_ui (`self.Pause UI`))
  (if (not (`KismetSystemLibrary.IsValid` (`self.Pause UI`)))
    (bind _returnvalue_2 (`|CreateWidget` "/Game/UI/WBP_PauseMenu.WBP_PauseMenu_C"))
    (set `self.Pause UI` _returnvalue_2))
  (if (`Widget.IsInViewport` (`self.Pause UI`))
    (`Widget.RemoveFromParent` _pause_ui)
    (`WidgetBlueprintLibrary.SetInputMode_GameOnly` _returnvalue)
    (else
      (`UserWidget.AddToViewport` _pause_ui 0)
      (`WidgetBlueprintLibrary.SetInputMode_GameAndUIEx` _returnvalue (`self.Pause UI`)))))

(event `Select Or Place Building`
  (if (and (`KismetArrayLibrary.Array_IsEmpty` (`self.Tower Inventory`)) (`KismetArrayLibrary.Array_IsEmpty` (`self.MineInventory`)) (`KismetArrayLibrary.Array_IsEmpty` (`self.SawmillInventory`)))
    (`KismetSystemLibrary.PrintString` "All Empty")
    (elif (`KismetArrayLibrary.Array_IsNotEmpty` (`self.Tower Inventory`))
      (`self.PlaceBaseTowerBuilding`)
      (`GameplayStatics.PlaySound2D` "/Game/SFX/Tour_posé.Tour_posé" 1.0 1.0 0.0 null null)
      (elif (`KismetArrayLibrary.Array_IsNotEmpty` (`self.SawmillInventory`))
        (`self.PlaceSawmillBuilding`)
        (`GameplayStatics.PlaySound2D` "/Game/SFX/Scierie_posé.Scierie_posé" 1.0 1.0 0.0 null null)
        (elif (`KismetArrayLibrary.Array_IsNotEmpty` (`self.MineInventory`))
          (`self.PlaceMineBuilding`)
          (`GameplayStatics.PlaySound2D` "/Game/SFX/Mine_posé.Mine_posé" 1.0 1.0 0.0 null null))))))

(event `Toggle Shop`
  (bind _returnvalue (`GameplayStatics.GetPlayerController` 0))
  (bind _shop_ui (`self.Shop UI`))
  (if (not (`KismetSystemLibrary.IsValid` (`self.Shop UI`)))
    (bind _returnvalue_2 (`|CreateWidget` "/Game/UI/WBP_BuyingMenu.WBP_BuyingMenu_C"))
    (set `self.Shop UI` _returnvalue_2))
  (if (`Widget.IsInViewport` (`self.Shop UI`))
    (`Widget.RemoveFromParent` _shop_ui)
    (`WidgetBlueprintLibrary.SetInputMode_GameOnly` _returnvalue)
    (else
      (`UserWidget.AddToViewport` _shop_ui 0)
      (`WidgetBlueprintLibrary.SetInputMode_GameAndUIEx` _returnvalue (`self.Shop UI`)))))

(fn `ClearAllInventory`
  (`KismetArrayLibrary.Array_Clear` (`self.Tower Inventory`))
  (`KismetArrayLibrary.Array_Clear` (`self.MineInventory`))
  (`KismetArrayLibrary.Array_Clear` (`self.SawmillInventory`)))

(fn `PlaceBaseTowerBuilding`
  (bind (_worldlocation _worlddirection) (`PlayerController.DeprojectMousePositionToWorld` (`GameplayStatics.GetPlayerController` 0)))
  (bind _towerinformation (`/Game/Actors/Manager/BP_LevelManager.TowerInformation` (`self.LevelInformation`)))
  (bind _basetower (`/Game/Actors/Manager/BP_TowerManager.BaseTower` _towerinformation))
  (bind _outhit (`KismetSystemLibrary.LineTraceSingle` :`Start` _worldlocation :`End` (* _worlddirection (`self.Range`)) :`TraceChannel` "TraceTypeQuery2" :`DrawDebugType` "ForDuration"))
  (bind (_bblockinghit _binitialoverlap _time _distance _location _impactpoint _normal _impactnormal _physmat _hitactor) (`GameplayStatics.BreakHitResult` _outhit))
  (if (`self.ActorHasTag` _hitactor "Tile")
    (bind _tile (`/Game/Actors/Manager/BP_TilesManager.FindTheRightTile` (`/Game/Actors/Manager/BP_LevelManager.TilesInformations` (`self.LevelInformation`)) (`KismetSystemLibrary.GetDisplayName` _hitactor)))
    (bind _ac_statetile (`/Game/Actors/Tiles/BP_Tiles.AC_StateTile` _tile))
    (bind _returnvalue (`/Game/Actors/Tiles/AC_StateTile.Is` _ac_statetile "OCCUPY" "NewEnumerator4"))
    (if _returnvalue
      (`/Game/Actors/Tiles/AC_StateTile.Change` _ac_statetile "OCCUPY" "NewEnumerator1")
      (bind _returnvalue_2 (`|SpawnActorFromClass` (`|GetArrayItem` (`self.Tower Inventory`)) (`self.GetTransform` _tile) "AlwaysSpawn" "MultiplyWithRoot" null null))
      (bind _returnvalue_3 (`KismetArrayLibrary.Array_Add` _basetower _returnvalue_2))
      (`KismetArrayLibrary.Array_Add` (`/Game/Actors/Manager/BP_TowerManager.AllTower` _towerinformation) _returnvalue_2)
      (set `/Game/Actors/Tower/BP_BaseTower.Position` (`/Game/Actors/Tiles/BP_Tiles.TilePosition` _tile) (`|GetArrayItem` _basetower _returnvalue_3))
      (`self.ClearAllInventory`))))

(fn `PlaceMineBuilding`
  (bind (_worldlocation _worlddirection) (`PlayerController.DeprojectMousePositionToWorld` (`GameplayStatics.GetPlayerController` 0)))
  (bind _ressourcesinformation (`/Game/Actors/Manager/BP_LevelManager.RessourcesInformation` (`self.LevelInformation`)))
  (bind _mine (`/Game/Actors/Manager/BP_RessourcesManager.Mine` _ressourcesinformation))
  (bind _outhit (`KismetSystemLibrary.LineTraceSingle` :`Start` _worldlocation :`End` (* _worlddirection (`self.Range`)) :`TraceChannel` "TraceTypeQuery2" :`DrawDebugType` "ForDuration"))
  (bind (_bblockinghit _binitialoverlap _time _distance _location _impactpoint _normal _impactnormal _physmat _hitactor) (`GameplayStatics.BreakHitResult` _outhit))
  (if (`self.ActorHasTag` _hitactor "Tile")
    (bind _tile (`/Game/Actors/Manager/BP_TilesManager.FindTheRightTile` (`/Game/Actors/Manager/BP_LevelManager.TilesInformations` (`self.LevelInformation`)) (`KismetSystemLibrary.GetDisplayName` _hitactor)))
    (bind _ac_statetile (`/Game/Actors/Tiles/BP_Tiles.AC_StateTile` _tile))
    (bind _returnvalue (`/Game/Actors/Tiles/AC_StateTile.Is` _ac_statetile "OCCUPY" "NewEnumerator4"))
    (if _returnvalue
      (`/Game/Actors/Tiles/AC_StateTile.Change` _ac_statetile "OCCUPY" "NewEnumerator3")
      (bind _returnvalue_2 (`|SpawnActorFromClass` (`|GetArrayItem` (`self.MineInventory`)) (`self.GetTransform` _tile) "AlwaysSpawn" "MultiplyWithRoot" null null))
      (bind _returnvalue_3 (`KismetArrayLibrary.Array_Add` _mine _returnvalue_2))
      (`KismetArrayLibrary.Array_Add` (`/Game/Actors/Manager/BP_RessourcesManager.AllBuilding` _ressourcesinformation) _returnvalue_2)
      (set `/Game/Actors/Ressources/BP_Mine.Position` (`/Game/Actors/Tiles/BP_Tiles.TilePosition` _tile) (`|GetArrayItem` _mine _returnvalue_3))
      (`self.ClearAllInventory`))))

(fn `PlaceSawmillBuilding`
  (bind (_worldlocation _worlddirection) (`PlayerController.DeprojectMousePositionToWorld` (`GameplayStatics.GetPlayerController` 0)))
  (bind _ressourcesinformation (`/Game/Actors/Manager/BP_LevelManager.RessourcesInformation` (`self.LevelInformation`)))
  (bind _sawmill (`/Game/Actors/Manager/BP_RessourcesManager.Sawmill` _ressourcesinformation))
  (bind _outhit (`KismetSystemLibrary.LineTraceSingle` :`Start` _worldlocation :`End` (* _worlddirection (`self.Range`)) :`TraceChannel` "TraceTypeQuery2" :`DrawDebugType` "ForDuration"))
  (bind (_bblockinghit _binitialoverlap _time _distance _location _impactpoint _normal _impactnormal _physmat _hitactor) (`GameplayStatics.BreakHitResult` _outhit))
  (if (`self.ActorHasTag` _hitactor "Tile")
    (bind _tile (`/Game/Actors/Manager/BP_TilesManager.FindTheRightTile` (`/Game/Actors/Manager/BP_LevelManager.TilesInformations` (`self.LevelInformation`)) (`KismetSystemLibrary.GetDisplayName` _hitactor)))
    (bind _ac_statetile (`/Game/Actors/Tiles/BP_Tiles.AC_StateTile` _tile))
    (bind _returnvalue (`/Game/Actors/Tiles/AC_StateTile.Is` _ac_statetile "OCCUPY" "NewEnumerator4"))
    (if _returnvalue
      (`/Game/Actors/Tiles/AC_StateTile.Change` _ac_statetile "OCCUPY" "NewEnumerator3")
      (bind _returnvalue_2 (`|SpawnActorFromClass` (`|GetArrayItem` (`self.SawmillInventory`)) (`self.GetTransform` _tile) "AlwaysSpawn" "MultiplyWithRoot" null null))
      (bind _returnvalue_3 (`KismetArrayLibrary.Array_Add` _sawmill _returnvalue_2))
      (`KismetArrayLibrary.Array_Add` (`/Game/Actors/Manager/BP_RessourcesManager.AllBuilding` _ressourcesinformation) _returnvalue_2)
      (set `/Game/Actors/Ressources/BP_Mine.Position` (`/Game/Actors/Tiles/BP_Tiles.TilePosition` _tile) (`|GetArrayItem` _sawmill _returnvalue_3))
      (`self.ClearAllInventory`))))

(fn `Select Shop Tower Building`
  (`self.ClearAllInventory`)
  (`KismetArrayLibrary.Array_Add` (`self.Tower Inventory`) "/Game/Actors/Tower/BP_BaseTower.BP_BaseTower_C"))

(fn `SelectBaseTowerBuilding`
  (bind (_worldlocation _worlddirection) (`PlayerController.DeprojectMousePositionToWorld` (`GameplayStatics.GetPlayerController` 0)))
  (`KismetArrayLibrary.Array_Clear` (`self.Tower Inventory`))
  (bind _outhit (`KismetSystemLibrary.LineTraceSingle` :`Start` _worldlocation :`End` (* _worlddirection (`self.Range`)) :`TraceChannel` "TraceTypeQuery2" :`DrawDebugType` "ForDuration"))
  (if (`self.ActorHasTag` (`.HitActor` (`GameplayStatics.BreakHitResult` _outhit)) "BaseTower")
    (`KismetArrayLibrary.Array_Add` (`self.Tower Inventory`) "/Game/Actors/Tower/BP_BaseTower.BP_BaseTower_C")))

(fn `SelectMineShop`
  (`self.ClearAllInventory`)
  (`KismetArrayLibrary.Array_Add` (`self.MineInventory`) "/Game/Actors/Ressources/BP_Mine.BP_Mine_C"))

(fn `SelectSawmillShop`
  (`self.ClearAllInventory`)
  (`KismetArrayLibrary.Array_Add` (`self.SawmillInventory`) "/Game/Actors/Ressources/BP_Sawmill.BP_Sawmill_C"))

(fn `Toggle Upgrade UI`
  (bind _returnvalue (`GameplayStatics.GetPlayerController` 0))
  (bind _upgrade_ui (`self.Upgrade UI`))
  (bind (_worldlocation _worlddirection) (`PlayerController.DeprojectMousePositionToWorld` (`GameplayStatics.GetPlayerController` 0)))
  (bind _outhit (`KismetSystemLibrary.LineTraceSingle` :`Start` _worldlocation :`End` (* _worlddirection (`self.Range`)) :`TraceChannel` "TraceTypeQuery2" :`DrawDebugType` "ForDuration"))
  (if (`self.ActorHasTag` (`.HitActor` (`GameplayStatics.BreakHitResult` _outhit)) "BaseTower")
    (if (not (`KismetSystemLibrary.IsValid` (`self.Upgrade UI`)))
      (bind _returnvalue_2 (`|CreateWidget` "/Game/UI/WBP_UpgradeMenu.WBP_UpgradeMenu_C" (`GameplayStatics.GetPlayerController` 0)))
      (set `self.Upgrade UI` _returnvalue_2))
    (if (`Widget.IsInViewport` (`self.Upgrade UI`))
      (`Widget.RemoveFromParent` _upgrade_ui)
      (`WidgetBlueprintLibrary.SetInputMode_GameOnly` _returnvalue)
      (else
        (`UserWidget.AddToViewport` _upgrade_ui 0)
        (`WidgetBlueprintLibrary.SetInputMode_GameAndUIEx` _returnvalue (`self.Upgrade UI`))))))

(fn `UserConstructionScript`)