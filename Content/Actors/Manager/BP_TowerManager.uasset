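; Tower manager for a tile-based defense game that resolves tower attacks and removes destroyed towers from their type arrays with a sound.
; Base and catapult attacks offset the tower's tile index, check the OCCUPY state, damage enemies there, and queue kills in DeadEnemy.
; Catapult splash on neighboring tiles is nested inside the center-kill branch and queues those neighbors as dead regardless of health.
; Straight towers only compute target tiles, and large towers have no attack here.
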(fn `AttackBaseTower`
  (bind _tiles (`/Game/Actors/Manager/BP_TilesManager.Tiles` (`/Game/Actors/Manager/BP_LevelManager.TilesInformations` (`self.LevelInformations`))))
  (if (and (`KismetArrayLibrary.Array_IsNotEmpty` (`self.BaseTower`)) (`KismetArrayLibrary.Array_IsNotEmpty` (`/Game/Actors/Manager/BP_SpawnManager.AllEnemy` (`/Game/Actors/Manager/BP_LevelManager.SpawnInformation` (`self.LevelInformations`)))))
    (for _array_element (`self.BaseTower`)
      (bind _position (`/Game/Actors/Tower/BP_BaseTower.Position` _array_element))
      (set `/Game/Actors/Tower/BP_BaseTower.FirstTileAttack` (+ _position 1) _array_element)
      (set `/Game/Actors/Tower/BP_BaseTower.SecondTileAttack` (+ _position 2) _array_element)
      (bind _output (`|GetArrayItem` _tiles (`/Game/Actors/Tower/BP_BaseTower.FirstTileAttack` _array_element)))
      (bind _returnvalue (`/Game/Actors/Tiles/AC_StateTile.Is` (`/Game/Actors/Tiles/BP_Tiles.AC_StateTile` _output) "OCCUPY" "NewEnumerator2"))
      (if _returnvalue
        (for _array_element_2 (`/Game/Actors/Manager/BP_SpawnManager.AllEnemy` (`/Game/Actors/Manager/BP_LevelManager.SpawnInformation` (`self.LevelInformations`)))
          (if (== (`/Game/Character/Enemy/BP_BasicEnemy.Position` _array_element_2) (`/Game/Actors/Tiles/BP_Tiles.TilePosition` _output))
            (bind _output_get (set `/Game/Character/Enemy/BP_BasicEnemy.Health` (- (`/Game/Character/Enemy/BP_BasicEnemy.Health` _array_element_2) (`self.GetBaseTowerDamage`)) _array_element_2))
            (if (<= _output_get 0)
              (`KismetArrayLibrary.Array_Add` (`/Game/Actors/Manager/BP_SpawnManager.DeadEnemy` (`/Game/Actors/Manager/BP_LevelManager.SpawnInformation` (`self.LevelInformations`))) _array_element_2)
              (`/Game/Actors/Tiles/AC_StateTile.Change` (`/Game/Actors/Tiles/BP_Tiles.AC_StateTile` _output) "OCCUPY" "NewEnumerator4")))))
      (bind _output_2 (`|GetArrayItem` _tiles (`/Game/Actors/Tower/BP_BaseTower.SecondTileAttack` _array_element)))
      (bind _returnvalue_2 (`/Game/Actors/Tiles/AC_StateTile.Is` (`/Game/Actors/Tiles/BP_Tiles.AC_StateTile` _output_2) "OCCUPY" "NewEnumerator2"))
      (if _returnvalue_2
        (for _array_element_3 (`/Game/Actors/Manager/BP_SpawnManager.AllEnemy` (`/Game/Actors/Manager/BP_LevelManager.SpawnInformation` (`self.LevelInformations`)))
          (if (== (`/Game/Character/Enemy/BP_BasicEnemy.Position` _array_element_3) (`/Game/Actors/Tiles/BP_Tiles.TilePosition` _output_2))
            (bind _output_get_2 (set `/Game/Character/Enemy/BP_BasicEnemy.Health` (- (`/Game/Character/Enemy/BP_BasicEnemy.Health` _array_element_3) (`self.GetBaseTowerDamage`)) _array_element_3))
            (if (<= _output_get_2 0)
              (`KismetArrayLibrary.Array_Add` (`/Game/Actors/Manager/BP_SpawnManager.DeadEnemy` (`/Game/Actors/Manager/BP_LevelManager.SpawnInformation` (`self.LevelInformations`))) _array_element_3)
              (`/Game/Actors/Tiles/AC_StateTile.Change` (`/Game/Actors/Tiles/BP_Tiles.AC_StateTile` _output_2) "OCCUPY" "NewEnumerator4"))))))))

(fn `AttackCatapultTower`
  (bind _tiles (`/Game/Actors/Manager/BP_TilesManager.Tiles` (`/Game/Actors/Manager/BP_LevelManager.TilesInformations` (`self.LevelInformations`))))
  (if (and (`KismetArrayLibrary.Array_IsNotEmpty` (`self.CatapultTower`)) (`KismetArrayLibrary.Array_IsNotEmpty` (`/Game/Actors/Manager/BP_SpawnManager.AllEnemy` (`/Game/Actors/Manager/BP_LevelManager.SpawnInformation` (`self.LevelInformations`)))))
    (for _array_element (`self.CatapultTower`)
      (bind _position (`/Game/Actors/Tower/BP_BaseTower.Position` _array_element))
      (set `/Game/Actors/Tower/BP_BaseTower.SecondTileAttack` (+ _position 2) _array_element)
      (set `/Game/Actors/Tower/BP_BaseTower.Third TileAttack` (+ _position 3) _array_element)
      (set `/Game/Actors/Tower/BP_BaseTower.FourthTileAttack` (+ _position 4) _array_element)
      (set `/Game/Actors/Tower/BP_BaseTower.FifhtTileAttack` (+ _position 5) _array_element)
      (set `/Game/Actors/Tower/BP_BaseTower.SixthTileAttack` (+ _position 6) _array_element)
      (bind _third_tileattack (`/Game/Actors/Tower/BP_BaseTower.Third TileAttack` _array_element))
      (`self.Catapult Zone Dmg` (`|GetArrayItem` _tiles _third_tileattack))
      (bind _result (`/Engine/EditorBlueprintResources/StandardMacros.IncrementInt` _third_tileattack)
        (:`  `
          (set `/Game/Actors/Tower/BP_BaseTower.HiddenTile` _result _array_element)
          (bind _hiddentile (`/Game/Actors/Tower/BP_BaseTower.HiddenTile` _array_element))
          (`self.Catapult Zone Dmg` (`|GetArrayItem` _tiles _hiddentile))
          (bind _result_2 (`/Engine/EditorBlueprintResources/StandardMacros.IncrementInt` _third_tileattack)
            (:`  `
              (set `/Game/Actors/Tower/BP_BaseTower.HiddenTile` _result_2 _array_element)
              (`self.Catapult Zone Dmg` (`|GetArrayItem` _tiles _hiddentile)))))))))

(fn `AttackStraightTower`
  (if (and (`KismetArrayLibrary.Array_IsNotEmpty` (`self.StraightTower`)) (`KismetArrayLibrary.Array_IsNotEmpty` (`/Game/Actors/Manager/BP_SpawnManager.AllEnemy` (`/Game/Actors/Manager/BP_LevelManager.SpawnInformation` (`self.LevelInformations`)))))
    (for _array_element (`self.StraightTower`)
      (bind _position (`/Game/Actors/Tower/BP_BaseTower.Position` _array_element))
      (set `/Game/Actors/Tower/BP_BaseTower.SecondTileAttack` (+ _position 2) _array_element)
      (set `/Game/Actors/Tower/BP_BaseTower.Third TileAttack` (+ _position 3) _array_element)
      (set `/Game/Actors/Tower/BP_BaseTower.FourthTileAttack` (+ _position 4) _array_element)
      (set `/Game/Actors/Tower/BP_BaseTower.FifhtTileAttack` (+ _position 5) _array_element)
      (set `/Game/Actors/Tower/BP_BaseTower.SixthTileAttack` (+ _position 6) _array_element))))

(fn `Catapult Zone Dmg`
  (params (InputPin :type "/Game/Actors/Tiles/BP_Tiles Object Reference"))
  (bind _returnvalue (`/Game/Actors/Tiles/AC_StateTile.Is` (`/Game/Actors/Tiles/BP_Tiles.AC_StateTile` InputPin) "OCCUPY" "NewEnumerator2"))
  (if _returnvalue
    (for _array_element (`/Game/Actors/Manager/BP_SpawnManager.AllEnemy` (`/Game/Actors/Manager/BP_LevelManager.SpawnInformation` (`self.LevelInformations`)))
      (if (== (`/Game/Character/Enemy/BP_BasicEnemy.Position` _array_element) (`/Game/Actors/Tiles/BP_Tiles.TilePosition` InputPin))
        (bind _output_get (set `/Game/Character/Enemy/BP_BasicEnemy.Health` (- (`/Game/Character/Enemy/BP_BasicEnemy.Health` _array_element) 3) _array_element))
        (if (<= _output_get 0)
          (`KismetArrayLibrary.Array_Add` (`/Game/Actors/Manager/BP_SpawnManager.DeadEnemy` (`/Game/Actors/Manager/BP_LevelManager.SpawnInformation` (`self.LevelInformations`))) _array_element)
          (`/Game/Actors/Tiles/AC_StateTile.Change` (`/Game/Actors/Tiles/BP_Tiles.AC_StateTile` InputPin) "OCCUPY" "NewEnumerator4")
          (for _array_element_2 (`/Game/Actors/Manager/BP_SpawnManager.AllEnemy` (`/Game/Actors/Manager/BP_LevelManager.SpawnInformation` (`self.LevelInformations`)))
            (if (== (`/Game/Character/Enemy/BP_BasicEnemy.Position` _array_element_2) (- (`/Game/Actors/Tiles/BP_Tiles.TilePosition` InputPin) 1))
              (set `/Game/Character/Enemy/BP_BasicEnemy.Health` (- (`/Game/Character/Enemy/BP_BasicEnemy.Health` _array_element_2) 1) _array_element_2)
              (`KismetArrayLibrary.Array_Add` (`/Game/Actors/Manager/BP_SpawnManager.DeadEnemy` (`/Game/Actors/Manager/BP_LevelManager.SpawnInformation` (`self.LevelInformations`))) _array_element_2)
              (`/Game/Actors/Tiles/AC_StateTile.Change` (`/Game/Actors/Tiles/BP_Tiles.AC_StateTile` InputPin) "OCCUPY" "NewEnumerator4")
              (for _array_element_3 (`/Game/Actors/Manager/BP_SpawnManager.AllEnemy` (`/Game/Actors/Manager/BP_LevelManager.SpawnInformation` (`self.LevelInformations`)))
                (if (== (`/Game/Character/Enemy/BP_BasicEnemy.Position` _array_element_3) (+ (`/Game/Actors/Tiles/BP_Tiles.TilePosition` InputPin) 1))
                  (set `/Game/Character/Enemy/BP_BasicEnemy.Health` (- (`/Game/Character/Enemy/BP_BasicEnemy.Health` _array_element_3) 1) _array_element_3)
                  (`KismetArrayLibrary.Array_Add` (`/Game/Actors/Manager/BP_SpawnManager.DeadEnemy` (`/Game/Actors/Manager/BP_LevelManager.SpawnInformation` (`self.LevelInformations`))) _array_element_3)
                  (`/Game/Actors/Tiles/AC_StateTile.Change` (`/Game/Actors/Tiles/BP_Tiles.AC_StateTile` InputPin) "OCCUPY" "NewEnumerator4"))))))))))

(fn `GetBaseTowerDamage`
  (returns (damage :type Integer))
  (return (`/Game/Actors/Tower/BP_BaseTower.damage` (`|GetArrayItem` (`self.BaseTower`)))))

(fn `RemoveAndDestroyDeadTowerFromTheRightArray`
  (params (DeadTower :type "/Game/Actors/Tower/BP_BaseTower Object Reference (by ref)"))
  (bind _straighttower (`self.StraightTower`))
  (bind _catapulttower (`self.CatapultTower`))
  (bind _largetower (`self.LargeTower`))
  (bind _basetower (`self.BaseTower`))
  (`KismetArrayLibrary.Array_RemoveItem` (`/Game/Actors/Manager/BP_TowerManager.AllTower` (`/Game/Actors/Manager/BP_LevelManager.TowerInformation` (`self.LevelInformations`))) DeadTower)
  (if (`KismetArrayLibrary.Array_Contains` _basetower DeadTower)
    (`KismetArrayLibrary.Array_RemoveItem` _basetower DeadTower)
    (`GameplayStatics.PlaySound2D` "/Game/SFX/Tour_cassé.Tour_cassé" 1.0 1.0 0.0 null null :!label _label)
    (`self.K2_DestroyActor` DeadTower)
    (elif (`KismetArrayLibrary.Array_Contains` _straighttower DeadTower)
      (`KismetArrayLibrary.Array_RemoveItem` _straighttower DeadTower)
      (goto _label)
      (elif (`KismetArrayLibrary.Array_Contains` _catapulttower DeadTower)
        (`KismetArrayLibrary.Array_RemoveItem` _catapulttower DeadTower)
        (goto _label)
        (elif (`KismetArrayLibrary.Array_Contains` _largetower DeadTower)
          (`KismetArrayLibrary.Array_RemoveItem` _largetower DeadTower)
          (goto _label))))))

(fn `UserConstructionScript`)